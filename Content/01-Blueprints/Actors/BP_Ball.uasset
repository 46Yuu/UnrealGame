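; Ball actor that changes its collision behavior while overlapping actors tagged HOLE.
; Sphere1's begin overlap switches its collision profile to Ball_Hole without updating overlaps, and end overlap restores Physicsactor with an overlap update.
; Both handlers skip the switch if the target profile is already set, and print the new profile name after a change.
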(event OnComponentBeginOverlap(Sphere1)
  (params (OverlappedComponent :type Primitive%20Component%20Object%20Reference) (OtherActor :type Actor%20Object%20Reference) (OtherComp :type Primitive%20Component%20Object%20Reference) (OtherBodyIndex :type Integer) (bFromSweep :type Boolean) (SweepResult :type Hit%20Result%20Structure%20%28by%20ref%29))
  (bind _sphere1 (Variables|Default|GetSphere1))
  (bind _returnvalue (Collision|GetCollisionProfileName _sphere1))
  (if (Actor|ActorHasTag OtherActor "HOLE")
    (if (not (== _returnvalue "Ball_Hole"))
      (Collision|SetCollisionProfileName _sphere1 "Ball_Hole" false :!class /Script/Engine.PrimitiveComponent)
      (Development|PrintText (Utilities|Text|ToText(Name) _returnvalue)))))

(event OnComponentEndOverlap(Sphere1)
  (params (OverlappedComponent :type Primitive%20Component%20Object%20Reference) (OtherActor :type Actor%20Object%20Reference) (OtherComp :type Primitive%20Component%20Object%20Reference) (OtherBodyIndex :type Integer))
  (bind _sphere1 (Variables|Default|GetSphere1))
  (bind _returnvalue (Collision|GetCollisionProfileName _sphere1))
  (if (Actor|ActorHasTag OtherActor "HOLE")
    (if (not (== _returnvalue "Physicsactor"))
      (Collision|SetCollisionProfileName _sphere1 "Physicsactor" true :!class /Script/Engine.PrimitiveComponent)
      (Development|PrintText (Utilities|Text|ToText(Name) _returnvalue)))))

(event EventBeginPlay)

(event Collision|EventActorBeginOverlap
  (params (OtherActor :type Actor%20Object%20Reference)))

(event EventTick
  (params (DeltaSeconds :type Float%20%28single-precision%29)))

(fn ConstructionScript)